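; Inspectable vase that counts as one objective for the first-person player.
; Interacting swaps input from player to vase, moves it before the camera and shows a text widget.
; Left-drag rotates it and the wheel changes camera distance; right-click restores input and starting transform, removes the widget and credits the objective once.
; BeginPlay raises the player's objective total; PickUpItem is defined but uncalled here.
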(event EventInteractwith
  (params (PlayerCharater :type BP%20First%20Person%20Character%20Object%20Reference))
  ;[1 1 1] Interact function - Xavier
  (bind _output_get (Variables|Default|SetPlayer%20Charater PlayerCharater))
  (Variables|/Game/Pre-Made_Assets/FirstPerson/Blueprints/BP_FirstPersonCharacter.BP_FirstPersonCharacter_C|GetItemCurHold _output_get
    (:then
      _)
    (:else
      _))
  (CallFunction|Inspect)
  (bind _returnvalue (UserInterface|CreateWidget "/Game/UI/UI_Interactable_Text_Vase.UI_Interactable_Text_Vase_C"))
  (UserInterface|Viewport|AddtoViewport _returnvalue 0))

(event EventBeginPlay
  (bind _mesh_0 (Variables|Default|GetMesh_0))
  ;[1 1 1] Count Total Objective Points - Xavier
  (Utilities|FlowControl|Sequence
    (:then_0
      (bind _asbp_first_person_character (Utilities|Casting|CastToBP_FirstPersonCharacter (Game|Player|GetPlayerPawn 0)))
      (Variables|/Game/Pre-Made_Assets/FirstPerson/Blueprints/BP_FirstPersonCharacter.BP_FirstPersonCharacter_C|SetMaxObjectives _asbp_first_person_character (+ (Variables|/Game/Pre-Made_Assets/FirstPerson/Blueprints/BP_FirstPersonCharacter.BP_FirstPersonCharacter_C|GetMaxObjectives _asbp_first_person_character) 1.0)))
    (:then_1
      (Variables|Default|SetInitialLocation (Transformation|GetWorldLocation _mesh_0))
      (Variables|Default|SetInitialRotation (Transformation|GetWorldRotation _mesh_0)))))

(event Input|MouseEvents|MouseX
  (params (AxisValue :type Float%20%28single-precision%29))
  ;[1 1 1] Rotate Item
  (if (Variables|Default|GetRotating)
    (Transformation|SetActorRotation (Math|Rotator|CombineRotators (Transformation|GetActorRotation) (Math|Rotator|MakeRotator 0.0 0.0 (* AxisValue -5.0))))))

(event Input|MouseEvents|MouseY
  (params (AxisValue :type Float%20%28single-precision%29))
  ;[1 1 1] Rotate Item
  (if (Variables|Default|GetRotating)
    (Transformation|SetActorRotation (Math|Rotator|CombineRotators (Transformation|GetActorRotation) (Math|Rotator|MakeRotator 0.0 (* AxisValue 5.0) 0.0)))))

(event Input|MouseEvents|LeftMouseButton
  (params (Key :type Key%20Structure :default "None"))
  ;[1 1 1] Rotate Item
  (:Pressed
    (Variables|Default|SetRotating true))
  (:Released
    (Variables|Default|SetRotating false)))

(event Input|MouseEvents|RightMouseButton
  (params (Key :type Key%20Structure :default "None"))
  (bind _player_charater (Variables|Default|GetPlayer%20Charater))
  ;[1 1 1] Stop interaction - Xavier
  (:Pressed
    (CallFunction|PutDownItem)
    (Input|EnableInput _player_charater (Game|GetPlayerController 0))
    (Input|DisableInput 0)
    (if (Variables|Default|GetInteracted)
      _
      (else
        (Variables|/Game/Pre-Made_Assets/FirstPerson/Blueprints/BP_FirstPersonCharacter.BP_FirstPersonCharacter_C|SetCurObjectives _player_charater (+ (Variables|/Game/Pre-Made_Assets/FirstPerson/Blueprints/BP_FirstPersonCharacter.BP_FirstPersonCharacter_C|GetCurObjectives _player_charater) 1.0))
        (Variables|Default|SetInteracted true)
        (Development|PrintString "Interacted")))
    (Transformation|SetActorLocationAndRotation (Variables|Default|GetInitialLocation) (Variables|Default|GetInitialRotation))
    (Widget|RemovefromParent (stale EventInteractwith _returnvalue))))

(event Input|MouseEvents|MouseWheelUp
  (params (Key :type Key%20Structure :default "None"))
  (bind _returnvalue (Game|GetPlayerCameraManager 0))
  ;[1 1 1] ZoomItem - Xavier
  ;;[1 1 1] Zoom In
  (:Pressed
    (bind _output_get (Variables|Default|SetZoomLevel (Math|Integer|Clamp(Integer) (+ (Variables|Default|GetZoomLevel) 1) 1 20)))
    (if (< _output_get 20)
      (Transformation|SetActorLocation (+ (Camera|GetCameraLocation _returnvalue) (* (Math|Vector|GetForwardVector (Camera|GetCameraRotation _returnvalue)) (* (Variables|Default|GetZoomLevel) 20))) false false))))

(event Input|MouseEvents|MouseWheelDown
  (params (Key :type Key%20Structure :default "None"))
  (bind _returnvalue (Game|GetPlayerCameraManager 0))
  ;[1 1 1] ZoomItem - Xavier
  ;;[1 1 1] Zoom Out
  (:Pressed
    (bind _output_get (Variables|Default|SetZoomLevel (Math|Integer|Clamp(Integer) (- (Variables|Default|GetZoomLevel) 1) 1 20)))
    (if (> _output_get 1)
      (Transformation|SetActorLocation (+ (Camera|GetCameraLocation _returnvalue) (* (Math|Vector|GetForwardVector (Camera|GetCameraRotation _returnvalue)) (* (Variables|Default|GetZoomLevel) 20))) false false))))

(fn ConstructionScript)

(fn PickUpItem
  (Transformation|AttachComponentToComponent (Variables|/Game/Pre-Made_Assets/FirstPerson/Blueprints/BP_FirstPersonCharacter.BP_FirstPersonCharacter_C|GetPickupAbility (Variables|Default|GetPlayer%20Charater)) "None" "KeepRelative" "KeepRelative" "KeepRelative" true)
  (Physics|SetSimulatePhysics (Variables|Default|GetMesh_0) false)
  (Collision|SetCollisionEnabled (Variables|Default|GetMesh_0) "NoCollision")
  (Variables|/Game/Pre-Made_Assets/FirstPerson/Blueprints/BP_FirstPersonCharacter.BP_FirstPersonCharacter_C|SetItemCurHold (Variables|Default|GetPlayer%20Charater) self))

(fn Inspect
  (bind _returnvalue (Game|GetPlayerController 0))
  (bind _returnvalue_2 (Game|GetPlayerCameraManager 0))
  (Input|DisableInput (Variables|Default|GetPlayer%20Charater) _returnvalue)
  (Input|EnableInput _returnvalue)
  (Transformation|SetActorLocation (+ (Camera|GetCameraLocation _returnvalue_2) (* (Math|Vector|GetForwardVector (Camera|GetCameraRotation _returnvalue_2)) "200.000000,200.000000,200.000000")) false false)
  (Collision|SetCollisionEnabled (Variables|Default|GetMesh_0) "NoCollision"))

(fn PutDownItem
  (bind _returnvalue (Game|GetPlayerCameraManager 0))
  (Collision|SetCollisionEnabled (Variables|Default|GetMesh_0) "QueryAndPhysics")
  (Transformation|DetachFromActor "KeepWorld" "KeepWorld" "KeepWorld")
  (Transformation|SetActorLocation (+ (Camera|GetCameraLocation _returnvalue) (* (Math|Vector|GetForwardVector (Camera|GetCameraRotation _returnvalue)) "200.000000,200.000000,200.000000")) false false))

(fn InteractDoor
  (params (interactorFunction :type Character%20Object%20Reference))
  (return false))