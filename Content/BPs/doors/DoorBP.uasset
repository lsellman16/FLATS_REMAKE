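; Interactable door Blueprint that swings open and shut, with a lock tied to the player character's AllObjectives flag.
; openDoor clears the lock when objectives are complete, then flip-flops a timeline lerping the mesh's yaw, or shows a locked-door widget.
; Leaving Box1 with objectives incomplete relocks and reverses the door.
; InteractDoor scales timeline speed before opening; its closing path is unconnected, and locked-door audio is only a debug print.
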(event OnComponentEndOverlap(Box1)
  (params (OverlappedComponent :type Primitive%20Component%20Object%20Reference) (OtherActor :type Actor%20Object%20Reference) (OtherComp :type Primitive%20Component%20Object%20Reference) (OtherBodyIndex :type Integer))
  (bind _asbp_first_person_character (Utilities|Casting|CastToBP_FirstPersonCharacter (Game|Player|GetPlayerPawn 0)))
  (if (not (Variables|/Game/Pre-Made_Assets/FirstPerson/Blueprints/BP_FirstPersonCharacter.BP_FirstPersonCharacter_C|GetAllObjectives _asbp_first_person_character))
    (Variables|Default|SetLocked true)
    (bind _door (Timeline|OpenDoor%20Timeline Reverse)
      (:Update
        (Transformation|SetRelativeRotation (Variables|Default|GetDoorSM) (Math|Rotator|MakeRotator 0.0 0.0 (Math|Float|Lerp (Variables|Default|GetopenPos) (Variables|Default|GetclosePos) _door)) false false)))))

(event Custom|openDoor
  (bind _asbp_first_person_character (Utilities|Casting|CastToBP_FirstPersonCharacter (Game|Player|GetPlayerPawn 0)))
  (bind _output_get (Variables|Default|SetAs%20BP%20First%20Person%20Character _asbp_first_person_character))
  (if (Variables|/Game/Pre-Made_Assets/FirstPerson/Blueprints/BP_FirstPersonCharacter.BP_FirstPersonCharacter_C|GetAllObjectives _output_get)
    (Variables|Default|SetLocked false))
  (if (Variables|Default|GetIsOpen?)
    (Development|PrintString "Play Locked Door Audio" :!label _label)
    (elif (Variables|Default|GetLocked)
      (Development|PrintString "Hello")
      (bind _returnvalue (UserInterface|CreateWidget "/Game/Widgets/UI/UI_Interactable_Door_Locked.UI_Interactable_Door_Locked_C"))
      (UserInterface|Viewport|AddtoViewport _returnvalue 0)
      (goto _label)
      (else
        (Utilities|FlowControl|FlipFlop
          (:A
            (bind _door (Timeline|OpenDoor%20Timeline Play)
              (:Update
                (Transformation|SetRelativeRotation (Variables|Default|GetDoorSM) (Math|Rotator|MakeRotator 0.0 0.0 (Math|Float|Lerp (Variables|Default|GetopenPos) (Variables|Default|GetclosePos) _door)) false false))))
          (:B
            (Timeline|OpenDoor%20Timeline Reverse)))))))

(fn ConstructionScript)

(fn InteractDoor
  (params (interactorFunction :type Character%20Object%20Reference))
  (if (not (Variables|Default|GetIsOpen?))
    (Components|Timeline|SetPlayRate (Variables|Default|GetOpenDoor%20Timeline) (/ 1.0 (Variables|Default|GettimeTakesToOpen%20%28sec%29)))
    (CallFunction|OpenDoor)
    (return true)))